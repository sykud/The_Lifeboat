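; Mario pawn that walks to one of three fixed map destinations in response to direction choices from the game instance.
; On BeginPlay it asks GameInfoInstance to show the choices and binds handlers to its go-north, go-east and go-west events.
; Each handler issues an AI MoveTo to hard-coded coordinates.
; The East and West bindings are crossed, calling the handlers named West and East respectively.
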(event Custom|AI_MoveToEast
  (AI|AIMoveTo (Pawn|GetControlledPawn (Pawn|GetController)) "-340.000000,310.000000, 0" 0 5.0 false))

(event Custom|AI_MoveToNorth
  (AI|AIMoveTo (Pawn|GetControlledPawn (Pawn|GetController)) "350.000000,350.000000, 0" 0 5.0 false))

(event Custom|AI_MoveToWest
  (AI|AIMoveTo (Pawn|GetControlledPawn (Pawn|GetController)) "-320.000000,-380.000000, 0" 0 5.0 false))

(event EventBeginPlay
  (bind _asgame_info_instance (Utilities|Casting|CastToGameInfoInstance (Game|GetGameInstance)))
  (Default|ShowChoices _asgame_info_instance)
  (EventDispatchers|BindEventtoMarioGoNorth _asgame_info_instance (delegate Custom|AI_MoveToNorth))
  (EventDispatchers|BindEventtoMarioGoEast _asgame_info_instance (delegate Custom|AI_MoveToWest))
  (EventDispatchers|BindEventtoMarioGoWest _asgame_info_instance (delegate Custom|AI_MoveToEast)))

(fn ConstructionScript)