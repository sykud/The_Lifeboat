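; BP_DayNightLight is a light actor that steps through a three-phase day, dusk and night color cycle.
; BeginPlay caches the GameInfoInstance game instance, which holds the current DayNight phase.
; Each RunDayNightCycle call tints the light white, orange or dark blue for that phase, then advances it.
; The night phase wraps back to day, increments the local NumberDay counter and prints it.
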(event EventBeginPlay
  (bind _asgame_info_instance (Utilities|Casting|CastToGameInfoInstance (Game|GetGameInstance)))
  (Variables|Default|SetGameInfoRef _asgame_info_instance))

(event EventTick
  (params (DeltaSeconds :type Float%20%28single-precision%29)))

(fn ConstructionScript)

(fn RunDayNightCycle
  (bind _gameinforef (Variables|Default|GetGameInfoRef))
  (switch int (Variables|/Game/GAME/Blueprints/AllLevels/GameInfoInstance.GameInfoInstance_C|GetDayNight (Variables|Default|GetGameInfoRef))
    (:0
      (Rendering|Components|Light|SetLightColor (Variables|Default|GetLightComponent) "(R=1.000000,G=1.000000,B=1.000000,A=1.000000)" true)
      (bind _result (Math|Integer|IncrementInt (Variables|/Game/GAME/Blueprints/AllLevels/GameInfoInstance.GameInfoInstance_C|GetDayNight _gameinforef) :!label _label)
        (:%20%20
          (Variables|/Game/GAME/Blueprints/AllLevels/GameInfoInstance.GameInfoInstance_C|SetDayNight _gameinforef _result))))
    (:1
      (Rendering|Components|Light|SetLightColor (Variables|Default|GetLightComponent) "(R=1.000000,G=0.209716,B=0.000000,A=1.000000)" true)
      (goto _label))
    (:2
      (Rendering|Components|Light|SetLightColor (Variables|Default|GetLightComponent) "(R=0.000000,G=0.058686,B=0.229167,A=1.000000)" true)
      (Variables|/Game/GAME/Blueprints/AllLevels/GameInfoInstance.GameInfoInstance_C|SetDayNight _gameinforef 0)
      (bind _result_2 (Math|Integer|IncrementInt (Variables|Default|GetNumberDay))
        (:%20%20
          (bind _output_get (Variables|Default|SetNumberDay _result_2))
          (Development|PrintString (Utilities|String|ToString(Integer) _output_get))))))
  (return))